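; ItemActor is an actor that displays an item's info in the world through a 3DItem widget.
; On BeginPlay it creates the widget from its ItemInfo and assigns it to its Widget component.
; On Tick, after a short Delay, it rotates its Sphere component to look at the first player's pawn if that pawn is valid.
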(event `self.ReceiveBeginPlay`
  (`parent.ReceiveBeginPlay`)
  (bind _returnvalue (`|CreateWidget` "/Game/ProStarter/Blueprint/UI/3DItem.3DItem_C" null (`self.ItemInfo`)))
  (`WidgetComponent.SetWidget` (`self.Widget`) _returnvalue))

(event `self.ReceiveTick`
  (params (DeltaSeconds :type "Float (single-precision)"))
  (bind _returnvalue (`GameplayStatics.GetPlayerPawn` 0))
  (`parent.ReceiveTick` DeltaSeconds)
  (`KismetSystemLibrary.Delay` 0.01)
  (`/Engine/EditorBlueprintResources/StandardMacros.IsValid` _returnvalue
    (:`Is Valid`
      (`SceneComponent.K2_SetWorldRotation` (`self.Sphere`) (`KismetMathLibrary.FindLookAtRotation` (`self.K2_GetActorLocation`) (`self.K2_GetActorLocation` _returnvalue)) false false))))

(fn `UserConstructionScript`
  (`parent.UserConstructionScript`))