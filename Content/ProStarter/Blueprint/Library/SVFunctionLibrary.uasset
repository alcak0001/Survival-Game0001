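; Blueprint function library for the item and wearable-container inventory, plus small server-type and local-character checks.
; Data table lookups by ItemID supply type, icon, stackability and capacity, while each item's AdditionList map holds per-instance values such as piece count.
; Wearable helpers compare, equip and unequip gear, and add or remove contents, merging or splitting stacks.
; Auto-placement tries four fixed wearable slots in order, splitting by free capacity and returning any remainder.
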(fn `Chance Weariable Item`
  (params (`Weariable Item` :type "Array of /Game/ProStarter/Data/Struct/WeariableItemInfo Structure") (`New Item` :type "/Game/ProStarter/Data/Struct/ItemInfo Structure (by ref)"))
  (returns (Successful :type Boolean) (Chance :type Boolean))
  (locals (`Remaing Item(Local)` :type "/Game/ProStarter/Data/Struct/ItemInfo Structure") (`Remaing Item IsValid(Local)` :type Boolean :default false))
  (bind (_successful _data) (`self.Get Weariable Item Data` `New Item`))
  (bind ((`Container?_19_C50A4D7E43662620701B8AAC90A3DA6F` _container_) (`MaxCapasity_13_0D153F2048C4AB312C8B2B88B4B2131F` _maxcapasity) (`WeariableArray_16_E5DB5DAB442B107399092BA8AA3F79C5` _weariablearray)) (break `/Game/ProStarter/Data/Struct/WeariableData` _data))
  (if _successful
    (if _container_
      (bind (_maxcapasity_2 _usablecapasity) (`self.Get Weariable Useable Capasity` (`|GetArrayItem` `Weariable Item` _weariablearray)))
      (if (>= _maxcapasity (- _maxcapasity_2 _usablecapasity))
        (return true true)
        (else
          (return true false)))
      (else
        (return true true)))
    (else
      (return false false))))

(fn `Create Item`
  (params (ID :type Name) (AdditionList :type "Map of /Game/ProStarter/Data/Enum/AdditionType Enum to Integer"))
  (returns (`Create Item` :type "/Game/ProStarter/Data/Struct/ItemInfo Structure"))
  (locals (`AdditionList(Local)` :type "Map of /Game/ProStarter/Data/Enum/AdditionType Enum to Integer") (`MakeMap(Local)` :type "Map of /Game/ProStarter/Data/Enum/AdditionType Enum to Integer"))
  (bind _additionlist_local_ (`local.AdditionList(Local)`))
  (set `local.MakeMap(Local)` (`|MakeMap` "NewEnumerator1" 1 "NewEnumerator2" 100000 "NewEnumerator3" 0 "NewEnumerator4" :!type "/Game/ProStarter/Data/Enum/AdditionType Enum"))
  (bind _keys (`BlueprintMapLibrary.Map_Keys` (`local.AdditionList`)))
  (for _array_element _keys
    (`BlueprintMapLibrary.Map_Add` (`local.MakeMap(Local)`) _array_element (`BlueprintMapLibrary.Map_Find` (`local.AdditionList`) _array_element)))
  (bind _returnvalue (`|GetDataTableRow` "/Game/ProStarter/Data/DataTable/ItemDataTable.ItemDataTable" (`local.ID`))
    (:`then`
      (bind ((`ItemID_2_8966B79D4AD7BBB3ADA93DA5731CD65F` _itemid) (`Name_24_ABC3CC7C44A0097070B760A4B4217890` _name) (`ShortName_25_AE2DB84A4E664113C09E5E82FA2518E1` _shortname) (`AdditionFeatureList_23_7559D3074AFD8015517BC592650CD0EE` _additionfeaturelist)) (break `/Game/ProStarter/Data/Struct/ItemData` _returnvalue))
      (for _array_element_2 _additionfeaturelist
        (bind (_value _returnvalue_2) (`BlueprintMapLibrary.Map_Find` (`local.MakeMap(Local)`) _array_element_2))
        (if _returnvalue_2
          (`BlueprintMapLibrary.Map_Add` _additionlist_local_ _array_element_2 _value)
          (else
            (`BlueprintMapLibrary.Map_Add` _additionlist_local_ _array_element_2))))
      (return (make `/Game/ProStarter/Data/Struct/ItemInfo` _itemid (`local.AdditionList(Local)`))))))

(fn `Equip  Weariable Item`
  (params (`Weariable Item` :type "Array of /Game/ProStarter/Data/Struct/WeariableItemInfo Structure") (`New Item` :type "/Game/ProStarter/Data/Struct/ItemInfo Structure (by ref)"))
  (returns (`Weariable Array` :type Integer) (`Remaing Item IsValid` :type Boolean) (`Remaing Item` :type "/Game/ProStarter/Data/Struct/ItemInfo Structure"))
  (locals (`Remaing Item(Local)` :type "/Game/ProStarter/Data/Struct/ItemInfo Structure") (`Remaing Item IsValid(Local)` :type Boolean :default false))
  (bind ((`Container?_19_C50A4D7E43662620701B8AAC90A3DA6F` _container_) (`WeariableArray_16_E5DB5DAB442B107399092BA8AA3F79C5` _weariablearray)) (break `/Game/ProStarter/Data/Struct/WeariableData` (`.Data` (`self.Get Weariable Item Data` `New Item`))))
  (bind _output (`|GetArrayItem` `Weariable Item` _weariablearray))
  (bind ((`Item_16_73306AE248B9C7E37964AC8CAFBE935D` _item)) (break `/Game/ProStarter/Data/Struct/WeariableItemInfo` _output))
  (if (`self.Get Weariable Item Data` _item)
    (set `local.Remaing Item(Local)` _item)
    (set `local.Remaing Item IsValid(Local)` true))
  (setmembers `/Game/ProStarter/Data/Struct/WeariableItemInfo` :`StructRef` _output :`Item` (`local.New Item`))
  (return _weariablearray (`local.Remaing Item IsValid(Local)`) (`local.Remaing Item(Local)`)))

(fn `Get Item Data`
  (params (Item :type "/Game/ProStarter/Data/Struct/ItemInfo Structure"))
  (returns (Successful :type Boolean) (Data :type "/Game/ProStarter/Data/Struct/ItemData Structure"))
  (bind _returnvalue (`|GetDataTableRow` "/Game/ProStarter/Data/DataTable/ItemDataTable.ItemDataTable" (`.ItemID_4_73306AE248B9C7E37964AC8CAFBE935D` (break `/Game/ProStarter/Data/Struct/ItemInfo` Item)))
    (:`then`
      (return true _returnvalue))
    (:`RowNotFound`
      (return false))))

(fn `Get Item Icon`
  (params (Item :type "/Game/ProStarter/Data/Struct/ItemInfo Structure"))
  (returns (Successful :type Boolean) (Icon :type "Texture2D Object Reference"))
  (bind (_successful _data) (`self.Get Item Data` Item))
  (if _successful
    (return true (`.Icon_15_D56C43F0490DE5139CCF9C8099955C5D` (break `/Game/ProStarter/Data/Struct/ItemData` _data)))
    (else
      (return false null))))

(fn `Get Item Piece`
  (params (Item :type "/Game/ProStarter/Data/Struct/ItemInfo Structure"))
  (returns (Successful :type Boolean) (Piece :type Integer))
  (if (`self.Get Item Stackable` Item)
    (return true (`BlueprintMapLibrary.Map_Find` (`.AdditionList_11_046AD9DD4D63F03F08D8FBBB7B05C286` (break `/Game/ProStarter/Data/Struct/ItemInfo` Item)) "NewEnumerator1"))
    (else
      (return false 1))))

(fn `Get Item Stackable`
  (params (Item :type "/Game/ProStarter/Data/Struct/ItemInfo Structure"))
  (returns (Stackable :type Boolean))
  (bind ((`ItemID_4_73306AE248B9C7E37964AC8CAFBE935D` _itemid)) (break `/Game/ProStarter/Data/Struct/ItemInfo` (`local.Item`)))
  (switch `/Game/ProStarter/Data/Enum/ItemType` (`.Item Type` (`self.Get Item Type` Item))
    (:`NewEnumerator1`
      (bind _returnvalue (`|GetDataTableRow` "/Game/ProStarter/Data/DataTable/ResourcesDataTable.ResourcesDataTable" _itemid)
        (:`then`
          (return (`.IsStack?_1_A92E2749460C8ED853E5CDAEDB4C099D` (break `/Game/ProStarter/Data/Struct/ResourcesData` _returnvalue))))
        (:`RowNotFound`
          _)))
    (:`NewEnumerator2`
      (bind _returnvalue_2 (`|GetDataTableRow` "/Game/ProStarter/Data/DataTable/UseableDataTable.UseableDataTable" _itemid)
        (:`then`
          (return (`.Stackable?_1_7E40F13144FBF8CCA0D158BC21FA3914` (break `/Game/ProStarter/Data/Struct/UseableData` _returnvalue_2))))
        (:`RowNotFound`
          _)))
    (:`NewEnumerator3`
      (return false))
    (:`NewEnumerator4`
      (return false))
    (:`NewEnumerator5`
      (return false)))
  (return false))

(fn `Get Item Type`
  (params (Item :type "/Game/ProStarter/Data/Struct/ItemInfo Structure"))
  (returns (Successful :type Boolean) (`Item Type` :type "/Game/ProStarter/Data/Enum/ItemType Enum"))
  (bind (_successful _data) (`self.Get Item Data` Item))
  (if _successful
    (return true (`.ItemType_16_DEE5D65F49A81064B737BAB8F5532C1D` (break `/Game/ProStarter/Data/Struct/ItemData` _data)))
    (else
      (return false "NewEnumerator0"))))

(fn `Get Item Use Capasity`
  (params (Item :type "/Game/ProStarter/Data/Struct/ItemInfo Structure"))
  (returns (`Multi Use Capasity` :type Integer) (`Single Use Capasity` :type Integer) (Piece :type Integer))
  (bind (_successful _piece) (`self.Get Item Piece` Item))
  (bind ((`UseCapasity_14_76D30A674AFD5362A2F9A8BC40BA4261` _usecapasity)) (break `/Game/ProStarter/Data/Struct/ItemData` (`.Data` (`self.Get Item Data` Item))))
  (return (* _usecapasity _piece) _usecapasity _piece))

(fn `Get Select Item`
  (params (`Weariable List` :type "Array of /Game/ProStarter/Data/Struct/WeariableItemInfo Structure") (`Container Array` :type Integer) (`Item Array` :type Integer))
  (returns (ContainerList :type "Array of /Game/ProStarter/Data/Struct/ItemInfo Structure") (Item :type "/Game/ProStarter/Data/Struct/ItemInfo Structure (by ref)"))
  (bind ((`ContainerList_15_AF13E52641CBE1442B7A0B893AE24EDE` _containerlist)) (break `/Game/ProStarter/Data/Struct/WeariableItemInfo` (`|GetArrayItem` `Weariable List` `Container Array`)))
  (return _containerlist (`|GetArrayItem` _containerlist `Item Array`)))

(fn `Get Weariable Container Empty`
  (params (`Weariable Item` :type "/Game/ProStarter/Data/Struct/WeariableItemInfo Structure (by ref)"))
  (returns (Empty :type Boolean))
  (bind (_item _containerlist) (break `/Game/ProStarter/Data/Struct/WeariableItemInfo` `Weariable Item`))
  (if (`.Container?` (`self.Get Weariable Container?` _item))
    (return (`KismetArrayLibrary.Array_IsEmpty` _containerlist))
    (else
      (return true))))

(fn `Get Weariable Container Same Item`
  (params (`Weariable Item` :type "/Game/ProStarter/Data/Struct/WeariableItemInfo Structure") (`New Item` :type "/Game/ProStarter/Data/Struct/ItemInfo Structure (by ref)"))
  (returns (Successful :type Boolean) (`Array Index` :type Integer) (Item :type "/Game/ProStarter/Data/Struct/ItemInfo Structure"))
  (locals (`İsValid(Local)` :type Boolean) (`Is Item(Local)` :type "/Game/ProStarter/Data/Struct/ItemInfo Structure") (`Is Array(Local)` :type Integer))
  (if (`self.Get Item Stackable` (`local.New Item`))
    (for (_array_element _array_index) (`.ContainerList_15_AF13E52641CBE1442B7A0B893AE24EDE` (break `/Game/ProStarter/Data/Struct/WeariableItemInfo` `Weariable Item`))
      (if (== (`.ItemID_4_73306AE248B9C7E37964AC8CAFBE935D` (break `/Game/ProStarter/Data/Struct/ItemInfo` _array_element)) (`.ItemID_4_73306AE248B9C7E37964AC8CAFBE935D` (break `/Game/ProStarter/Data/Struct/ItemInfo` (`local.New Item`))))
        (set `local.İsValid(Local)` true)
        (set `local.Is Item(Local)` _array_element)
        (set `local.Is Array(Local)` _array_index)))
    (return (`local.İsValid(Local)`) (`local.Is Array(Local)`) (`local.Is Item(Local)`))
    (else
      (return false 0))))

(fn `Get Weariable Container?`
  (params (ItemInfo :type "/Game/ProStarter/Data/Struct/ItemInfo Structure (by ref)"))
  (returns (Successful :type Boolean) (`Container?` :type Boolean) (MaxCapasity :type Integer))
  (bind (_successful _data) (`self.Get Weariable Item Data` ItemInfo))
  (bind ((`Container?_19_C50A4D7E43662620701B8AAC90A3DA6F` _container_) (`MaxCapasity_13_0D153F2048C4AB312C8B2B88B4B2131F` _maxcapasity)) (break `/Game/ProStarter/Data/Struct/WeariableData` _data))
  (return _successful _container_ _maxcapasity))

(fn `Get Weariable Item Compare`
  (params (`Weariable Item` :type "Array of /Game/ProStarter/Data/Struct/WeariableItemInfo Structure") (`New Item` :type "/Game/ProStarter/Data/Struct/ItemInfo Structure (by ref)"))
  (returns (Change :type Boolean))
  (bind (_successful _data) (`self.Get Weariable Item Data` (`.Item_16_73306AE248B9C7E37964AC8CAFBE935D` (break `/Game/ProStarter/Data/Struct/WeariableItemInfo` (`|GetArrayItem` `Weariable Item` (`.WeariableArray_16_E5DB5DAB442B107399092BA8AA3F79C5` (break `/Game/ProStarter/Data/Struct/WeariableData` (`.Data` (`self.Get Weariable Item Data` `New Item`)))))))))
  (if _successful
    (return (< (`.Priority_17_45DB84DA4C474A72226A718A0B03786C` (break `/Game/ProStarter/Data/Struct/WeariableData` _data)) (`.Priority_17_45DB84DA4C474A72226A718A0B03786C` (break `/Game/ProStarter/Data/Struct/WeariableData` (`.Data` (`self.Get Weariable Item Data` (`local.New Item`)))))))
    (else
      (return true))))

(fn `Get Weariable Item Data`
  (params (ItemInfo :type "/Game/ProStarter/Data/Struct/ItemInfo Structure (by ref)"))
  (returns (Successful :type Boolean) (Data :type "/Game/ProStarter/Data/Struct/WeariableData Structure"))
  (bind _returnvalue (`|GetDataTableRow` "/Game/ProStarter/Data/DataTable/WeariableDataTable.WeariableDataTable" (`.ItemID_4_73306AE248B9C7E37964AC8CAFBE935D` (break `/Game/ProStarter/Data/Struct/ItemInfo` ItemInfo)))
    (:`then`
      (return true _returnvalue))
    (:`RowNotFound`
      (return false))))

(fn `Get Weariable Useable Capasity`
  (params (`Weariable Item` :type "/Game/ProStarter/Data/Struct/WeariableItemInfo Structure (by ref)"))
  (returns (MaxCapasity :type Integer) (UsableCapasity :type Integer))
  (locals (`MaxCapasity(Local)` :type Integer :default 0) (`UsableCapasity(Local)` :type Integer :default 0))
  (bind (_item _containerlist) (break `/Game/ProStarter/Data/Struct/WeariableItemInfo` `Weariable Item`))
  (bind _output_get (set `local.MaxCapasity(Local)` (`.MaxCapasity` (`self.Get Weariable Container?` _item))))
  (set `local.UsableCapasity(Local)` _output_get)
  (for _array_element _containerlist
    (set `local.UsableCapasity(Local)` (- (`local.UsableCapasity(Local)`) (`self.Get Item Use Capasity` _array_element))))
  (return (`local.MaxCapasity(Local)`) (`local.UsableCapasity(Local)`)))

(fn `Inquiry TRY Weariable Added Item`
  (params (WeariableList :type "Array of /Game/ProStarter/Data/Struct/WeariableItemInfo Structure") (Item :type "/Game/ProStarter/Data/Struct/ItemInfo Structure"))
  (returns (Remaing :type Boolean) (`Remaing Item` :type "/Game/ProStarter/Data/Struct/ItemInfo Structure") (`Add Item List` :type "Array of /Game/ProStarter/Data/Struct/SelectContainerAddItem Structure"))
  (locals (`RemaingItem(Local)` :type "/Game/ProStarter/Data/Struct/ItemInfo Structure") (`Add Item List(Local)` :type "Array of /Game/ProStarter/Data/Struct/SelectContainerAddItem Structure"))
  (bind (_add _add_item _remaing _remaing_item) (`self.Inquiry Weariable Select Item Add` WeariableList 4 Item))
  (if _add
    (`KismetArrayLibrary.Array_Add` (`local.Add Item List(Local)`) (make `/Game/ProStarter/Data/Struct/SelectContainerAddItem` 4 _add_item))
    (if _remaing
      (bind (_add_2 _add_item_2 _remaing_2 _remaing_item_2) (`self.Inquiry Weariable Select Item Add` WeariableList 8 _remaing_item :!label _label))
      (if _add_2
        (`KismetArrayLibrary.Array_Add` (`local.Add Item List(Local)`) (make `/Game/ProStarter/Data/Struct/SelectContainerAddItem` 8 _add_item_2))
        (if _remaing_2
          (bind (_add_3 _add_item_3 _remaing_3 _remaing_item_3) (`self.Inquiry Weariable Select Item Add` WeariableList 6 _remaing_item_2 :!label _label_2))
          (if _add_3
            (`KismetArrayLibrary.Array_Add` (`local.Add Item List(Local)`) (make `/Game/ProStarter/Data/Struct/SelectContainerAddItem` 6 _add_item_3))
            (if _remaing_3
              (bind (_add_4 _add_item_4 _remaing_4 _remaing_item_4) (`self.Inquiry Weariable Select Item Add` WeariableList 3 _remaing_item_3 :!label _label_3))
              (if _add_4
                (`KismetArrayLibrary.Array_Add` (`local.Add Item List(Local)`) (make `/Game/ProStarter/Data/Struct/SelectContainerAddItem` 3 _add_item_4))
                (if _remaing_4
                  (return true _remaing_item_4 (`local.Add Item List(Local)`))
                  (else
                    _))
                (else
                  (return true _remaing_item_4 (`local.Add Item List(Local)`)))))
            (else
              (goto _label_3))))
        (else
          (goto _label_2))))
    (else
      (goto _label)))
  (return false (struct) (`local.Add Item List(Local)`)))

(fn `Inquiry Weariable Select Item Add`
  (params (WeariableList :type "Array of /Game/ProStarter/Data/Struct/WeariableItemInfo Structure") (`Weariable Array` :type Integer) (Item :type "/Game/ProStarter/Data/Struct/ItemInfo Structure"))
  (returns (Add :type Boolean) (`Add Item` :type "/Game/ProStarter/Data/Struct/ItemInfo Structure") (Remaing :type Boolean) (`Remaing Item` :type "/Game/ProStarter/Data/Struct/ItemInfo Structure"))
  (locals (`RemaingItem(Local)` :type "/Game/ProStarter/Data/Struct/ItemInfo Structure"))
  (bind _output (`|GetArrayItem` WeariableList `Weariable Array`))
  (bind (_multi_use_capasity _single_use_capasity) (`self.Get Item Use Capasity` (`local.Item`)))
  (bind (_successful _container_) (`self.Get Weariable Container?` (`.Item_16_73306AE248B9C7E37964AC8CAFBE935D` (break `/Game/ProStarter/Data/Struct/WeariableItemInfo` _output))))
  (if (and _successful _container_)
    (bind (_maxcapasity _usablecapasity) (`self.Get Weariable Useable Capasity` _output))
    (if (>= _usablecapasity _multi_use_capasity)
      (return true (`local.Item`) false)
      (else
        (bind _returnvalue (/ _usablecapasity _single_use_capasity))
        (if (<= 1 _returnvalue)
          (bind (_successful_2 _primary_item _remaing_item) (`self.Tool Item Divide` (`local.Item`) _returnvalue))
          (return true _primary_item true _remaing_item)
          (else
            (return false (struct) true (`local.Item`))))))
    (else
      (return false (struct) true (`local.Item`)))))

(fn `Item Add`
  (params (WeariableList :type "Array of /Game/ProStarter/Data/Struct/WeariableItemInfo Structure") (`Weariable Array` :type Integer) (Item :type "/Game/ProStarter/Data/Struct/ItemInfo Structure"))
  (returns (`Same Item` :type Boolean) (`Item Array` :type Integer))
  (locals (`RemaingItem(Local)` :type "/Game/ProStarter/Data/Struct/ItemInfo Structure"))
  (bind _output (`|GetArrayItem` WeariableList `Weariable Array`))
  (bind ((`ContainerList_15_AF13E52641CBE1442B7A0B893AE24EDE` _containerlist)) (break `/Game/ProStarter/Data/Struct/WeariableItemInfo` _output))
  (bind (_successful _array_index _item) (`self.Get Weariable Container Same Item` _output Item))
  (if _successful
    (`KismetArrayLibrary.Array_Set` _containerlist _array_index (`.Item` (`self.Tool Item Combine` _item (`local.Item`))))
    (return true _array_index)
    (else
      (`KismetArrayLibrary.Array_Add` _containerlist (`local.Item`))
      (return false 0))))

(fn `Item Remove`
  (params (WeariableList :type "Array of /Game/ProStarter/Data/Struct/WeariableItemInfo Structure") (`Weariable Array` :type Integer) (`Item Remove` :type Boolean) (`Item Array` :type Integer) (Item :type "/Game/ProStarter/Data/Struct/ItemInfo Structure"))
  (locals (`RemaingItem(Local)` :type "/Game/ProStarter/Data/Struct/ItemInfo Structure"))
  (bind ((`ContainerList_15_AF13E52641CBE1442B7A0B893AE24EDE` _containerlist)) (break `/Game/ProStarter/Data/Struct/WeariableItemInfo` (`|GetArrayItem` WeariableList `Weariable Array`)))
  (if (`local.Item Remove`)
    (`KismetArrayLibrary.Array_Remove` _containerlist (`local.Item Array`))
    (else
      (bind (_successful _primary_item _remaing_item) (`self.Tool Item Divide` (`|GetArrayItem` _containerlist (`local.Item Array`)) (`.Piece` (`self.Get Item Piece` (`local.Item`)))))
      (`KismetArrayLibrary.Array_Set` _containerlist (`local.Item Array`) _remaing_item)))
  (return))

(fn `SameCharacter`
  (params (`Pro Character` :type "/Game/ProStarter/Blueprint/Character/ProCharacter Object Reference"))
  (returns (SameCharacter :type Boolean))
  (bind _aspro_character (cast `/Game/ProStarter/Blueprint/Character/ProCharacter` (`GameplayStatics.GetPlayerCharacter` null)))
  (return (== _aspro_character (`local.Pro Character`))))

(fn `Server Type?`
  (params (__WorldContext :type "Object Object Reference"))
  (returns (`Server Type` :type "/Game/ProStarter/Data/Enum/ServerType Enum"))
  (if (`KismetSystemLibrary.IsDedicatedServer` null)
    (return "NewEnumerator0")
    (elif (`KismetSystemLibrary.IsServer` null)
      (return "NewEnumerator1")
      (else
        (return "NewEnumerator2")))))

(fn `Set  Item Piece`
  (params (Item :type "/Game/ProStarter/Data/Struct/ItemInfo Structure") (Piece :type "Integer (by ref)"))
  (returns (Successful :type Boolean))
  (if (`self.Get Item Stackable` Item)
    (`BlueprintMapLibrary.Map_Add` (`.AdditionList_11_046AD9DD4D63F03F08D8FBBB7B05C286` (break `/Game/ProStarter/Data/Struct/ItemInfo` (`local.Item`))) "NewEnumerator1" (`local.Piece`))
    (return true)
    (else
      (return false))))

(fn `Tool Item Combine`
  (params (`First Item` :type "/Game/ProStarter/Data/Struct/ItemInfo Structure") (`Second Item` :type "/Game/ProStarter/Data/Struct/ItemInfo Structure"))
  (returns (Successful :type Boolean) (Item :type "/Game/ProStarter/Data/Struct/ItemInfo Structure"))
  (locals (`Local Item` :type "/Game/ProStarter/Data/Struct/ItemInfo Structure"))
  (bind _output_get (set `local.Local Item` `First Item`))
  (`BlueprintMapLibrary.Map_Add` (`.AdditionList_11_046AD9DD4D63F03F08D8FBBB7B05C286` (break `/Game/ProStarter/Data/Struct/ItemInfo` _output_get)) "NewEnumerator1" (+ (`.Piece` (`self.Get Item Piece` `First Item`)) (`.Piece` (`self.Get Item Piece` `Second Item`))))
  (return true (`local.Local Item`)))

(fn `Tool Item Divide`
  (params (Item :type "/Game/ProStarter/Data/Struct/ItemInfo Structure") (Piece :type Integer))
  (returns (Successful :type Boolean) (`Primary Item` :type "/Game/ProStarter/Data/Struct/ItemInfo Structure") (`Remaing Item` :type "/Game/ProStarter/Data/Struct/ItemInfo Structure"))
  (locals (`Item (Local)` :type "/Game/ProStarter/Data/Struct/ItemInfo Structure") (`Remaing Item (Local)` :type "/Game/ProStarter/Data/Struct/ItemInfo Structure"))
  (bind _output_get (set `local.Item (Local)` Item))
  (set `local.Remaing Item (Local)` _output_get)
  (`BlueprintMapLibrary.Map_Add` (`.AdditionList_11_046AD9DD4D63F03F08D8FBBB7B05C286` (break `/Game/ProStarter/Data/Struct/ItemInfo` (`local.Item (Local)`))) "NewEnumerator1" (`local.Piece`))
  (`BlueprintMapLibrary.Map_Add` (`.AdditionList_11_046AD9DD4D63F03F08D8FBBB7B05C286` (break `/Game/ProStarter/Data/Struct/ItemInfo` (`local.Remaing Item (Local)`))) "NewEnumerator1" (- (`.Piece` (`self.Get Item Piece` (`local.Item`))) (`local.Piece`)))
  (return true (`local.Item (Local)`) (`local.Remaing Item (Local)`)))

(fn `UnEquip  Weariable Item`
  (params (`Weariable Item` :type "Array of /Game/ProStarter/Data/Struct/WeariableItemInfo Structure") (`Weariable Array` :type "Integer (by ref)"))
  (locals (`Remaing Item(Local)` :type "/Game/ProStarter/Data/Struct/ItemInfo Structure") (`Remaing Item IsValid(Local)` :type Boolean :default false))
  (`KismetArrayLibrary.Array_Set` `Weariable Item` `Weariable Array`)
  (return))